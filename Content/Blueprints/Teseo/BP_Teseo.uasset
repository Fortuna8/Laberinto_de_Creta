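; Teseo is a 2D flipbook player character for side-scrolling platforming, with running, sprinting and double jump through Enhanced Input.
; Movement follows the X axis, and the sign of acceleration flips the controller yaw to face left or right.
; Sprint switches max walk speed while held and records IsRunning.
; BeginPlay sets the idle flipbook and stores the spawn as Checkpoint, where Tick returns the character after falling below a height limit.
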(event `self.ReceiveBeginPlay`
  (bind _asplayer_controller (cast `PlayerController` (`self.GetController`)))
  (`EnhancedInputSubsystemInterface.AddMappingContext` (pcsubsystem `EnhancedInputLocalPlayerSubsystem` _asplayer_controller) "/Game/Entradas/NewInputMappingContext.NewInputMappingContext" 0 (struct))
  (`PaperFlipbookComponent.SetFlipbook` (`self.Sprite`) "/Game/Assets/Teseo/Idle/ModeloPersonajeV1__Idle.ModeloPersonajeV1__Idle")
  (set `self.checkpoint` (`self.K2_GetActorLocation`)))

(event `EnhancedInput|/Game/Entradas/Inputs/IA_Correr`
  (params (ActionValue :type "Float (double-precision)") (ElapsedSeconds :type "Float (double-precision)") (TriggeredSeconds :type "Float (double-precision)") (InputAction :type "InputAction Object Reference" :default "/Game/Entradas/Inputs/IA_Correr.IA_Correr"))
  (bind _returnvalue (`self.GetController`))
  (bind _returnvalue_x (`KismetMathLibrary.BreakVector` (`CharacterMovementComponent.GetCurrentAcceleration` (`self.CharacterMovement`))))
  ;[0.5991 1 0.8359] CORRER: Movimiento lateral base del personaje
  (:`Triggered`
    (`self.AddMovementInput` (1.0 0.0 0.0) ActionValue)
    ;[1 1 1] Determina la dirección al medir la aceleración del personaje (> o < que cero)
    (`/Engine/EditorBlueprintResources/StandardMacros.CompareFloat` _returnvalue_x
      (:`>`
        ;[1 1 1] Rotan el personaje en el eje Z (YAW)
        (`Controller.SetControlRotation` _returnvalue (`KismetMathLibrary.MakeRotator` 0.0)))
      (:`<`
        (`Controller.SetControlRotation` _returnvalue (`KismetMathLibrary.MakeRotator` 0.0 0.0 180.0))))))

(event `EnhancedInput|/Game/Entradas/Inputs/IA_Saltar`
  (params (ActionValue :type Boolean) (ElapsedSeconds :type "Float (double-precision)") (TriggeredSeconds :type "Float (double-precision)") (InputAction :type "InputAction Object Reference" :default "/Game/Entradas/Inputs/IA_Saltar.IA_Saltar"))
  ;[1 0.9451 0.349] SALTAR: Desplazamineto vertical.
  (:`Started`
    (`self.Jump`)
    (set `self.JumpMaxCount` 2)))

(event `EnhancedInput|/Game/Entradas/Inputs/IA_Sprint`
  (params (ActionValue :type Boolean) (ElapsedSeconds :type "Float (double-precision)") (TriggeredSeconds :type "Float (double-precision)") (InputAction :type "InputAction Object Reference" :default "/Game/Entradas/Inputs/IA_Sprint.IA_Sprint"))
  (bind _charactermovement (`self.CharacterMovement`))
  ;[0.5748 0.7806 1] SPRINT: Duplica la velocidad máxima al apretar Shift izquierdo y la reduce a la mitad al soltar.
  (:`Started`
    (set `self.bIsRunning` ActionValue)
    (set `CharacterMovementComponent.MaxWalkSpeed` 1000.0 _charactermovement))
  (:`Completed`
    (set `self.bIsRunning` ActionValue)
    (set `CharacterMovementComponent.MaxWalkSpeed` 600.0 _charactermovement)))

(event `self.ReceiveTick`
  (params (DeltaSeconds :type "Float (single-precision)"))
  (bind (_returnvalue_x _returnvalue_y _returnvalue_z) (`KismetMathLibrary.BreakVector` (`self.K2_GetActorLocation`)))
  ;[1 1 1] Respawn si el personaje se cae del mapa
  (if (<= _returnvalue_z -1700.0)
    (`self.K2_SetActorLocation` (`self.checkpoint`))))

(fn `UserConstructionScript`)